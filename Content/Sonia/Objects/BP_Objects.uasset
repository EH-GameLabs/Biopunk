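; BP_Objects is an object that shows an on-screen instruction widget while something overlaps its Sphere.
; Begin overlap prints a debug message, sets IsOverlapped and adds a new BP_ObjInstruction widget to the viewport; end overlap removes it and clears the flag.
; Any overlapping actor triggers this, as the third-person character cast is disconnected.
; Tick checks IsOverlapped but takes no action.
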(event `self.Sphere.OnComponentBeginOverlap`
  (params (OverlappedComponent :type "PrimitiveComponent Object Reference") (OtherActor :type "Actor Object Reference") (OtherComp :type "PrimitiveComponent Object Reference") (OtherBodyIndex :type Integer) (bFromSweep :type Boolean) (SweepResult :type "HitResult Structure (by ref)"))
  (`KismetSystemLibrary.PrintString` "collisione con oggetto")
  (set `self.IsOverlapped` true)
  (bind _returnvalue (`|CreateWidget` "/Game/Sonia/UI/BP_ObjInstruction.BP_ObjInstruction_C"))
  (`UserWidget.AddToViewport` _returnvalue 0))

(event `self.Sphere.OnComponentEndOverlap`
  (params (OverlappedComponent :type "PrimitiveComponent Object Reference") (OtherActor :type "Actor Object Reference") (OtherComp :type "PrimitiveComponent Object Reference") (OtherBodyIndex :type Integer))
  (`Widget.RemoveFromParent` (stale `self.Sphere.OnComponentBeginOverlap` _returnvalue))
  (set `self.IsOverlapped` false))

(event `Key|E`
  (params (Key :type "Key Structure")))

(event `self.ReceiveTick`
  (params (DeltaSeconds :type "Float (single-precision)"))
  (if (`self.IsOverlapped`)
    _))

(event `self.ReceiveBeginPlay`)

(fn `UserConstructionScript`)