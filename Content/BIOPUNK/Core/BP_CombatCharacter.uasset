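; BP_CombatCharacter is the player's combat character, adding hit feedback, target lock input and a Frenzy bar that scales combat performance.
; Dealing or taking damage plays camera shakes, with Niagara particles on damage taken, and raises or lowers the Frenzy bar.
; Bar changes update attack speed, combo availability and damage multiplier from that bar's stats, through a delegate handler named TEST.
; Target lock input prints debug text, and unconnected animation rate nodes remain.
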(event `self.DealtDamage`
  (params (Damage :type "Float (single-precision)") (ImpactPoint :type "Vector Structure (by ref)"))
  (bind _frenzy (`self.Frenzy`))
  ; Play effects when dealing and receiving damage
  (`GameplayStatics.PlayWorldCameraShake` "/Game/Variant_Combat/Blueprints/BP_CameraShake_Hit_Enemy.BP_CameraShake_Hit_Enemy_C" ImpactPoint 0.0 500.0)
  (`FrenzyComponent.IncreaseBar` _frenzy (`FrenzyComponent.IncreaseOnHit` _frenzy)))

(event `self.ReceivedDamage`
  (params (Damage :type "Float (single-precision)") (ImpactPoint :type "Vector Structure (by ref)") (DamageDirection :type "Vector Structure (by ref)"))
  (bind _frenzy (`self.Frenzy`))
  ; Play effects when dealing and receiving damage
  (`NiagaraFunctionLibrary.SpawnSystemAtLocation` "/Game/Variant_Combat/VFX/NS_Damage.NS_Damage" ImpactPoint (`KismetMathLibrary.Conv_VectorToRotator` DamageDirection))
  (`GameplayStatics.PlayWorldCameraShake` "/Game/Variant_Combat/Blueprints/BP_CameraShake_Hit_Player.BP_CameraShake_Hit_Player_C" ImpactPoint 0.0 500.0)
  (`FrenzyComponent.DecreaseBar` _frenzy (`FrenzyComponent.DecreaseOnTakeDamage` _frenzy)))

(event `EnhancedInput|/Game/BIOPUNK/Input/InputAction/IA_TargetLock`
  (params (ActionValue :type Boolean) (ElapsedSeconds :type "Float (double-precision)") (TriggeredSeconds :type "Float (double-precision)") (InputAction :type "InputAction Object Reference" :default "/Game/BIOPUNK/Input/InputAction/IA_TargetLock.IA_TargetLock"))
  (:`Triggered`
    (`KismetSystemLibrary.PrintString` "Trying to lock")
    (`self.ToggleTargetLock`)))

(event `self.ReceiveBeginPlay`
  (add `FrenzyComponent.OnBarChangedDelegate` (`self.Frenzy`) (delegate `TEST`))
  (set `self.BarDamage` (`.DamageMultiplier` (break `BarData` (`|GetArrayItem` (`FrenzyComponent.BarStats` (`self.Frenzy`)) (stale `TEST` index))))))

(event `TEST`
  (params (index :type Integer))
  (bind ((`DamageMultiplier` _damagemultiplier) (`AttackSpeedMultiplier` _attackspeedmultiplier) (`HasCombo` _hascombo)) (break `BarData` (`|GetArrayItem` (`FrenzyComponent.BarStats` (`self.Frenzy`)) index)))
  (set `self.AttackSpeed` _attackspeedmultiplier)
  (set `self.HasCombo` _hascombo)
  (set `self.BarDamage` _damagemultiplier))

(fn `UserConstructionScript`)