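; BP_Potion is a healing pickup that restores health immediately and respawns after a delay.
; Overlapping its sphere collision with a BP_TestingCharacter calls Interact, which adds HealAmount to that character's health component.
; SetActive then toggles visibility, collision and tick off, and back on after RespawnTime, reusing the same actor.
; An AddPotion call to the inventory subsystem remains in the graph but is disconnected.
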(event `self.Sphere Collision.OnComponentBeginOverlap`
  (params (OverlappedComponent :type "PrimitiveComponent Object Reference") (OtherActor :type "Actor Object Reference") (OtherComp :type "PrimitiveComponent Object Reference") (OtherBodyIndex :type Integer) (bFromSweep :type Boolean) (SweepResult :type "HitResult Structure (by ref)"))
  (bind _asbp_testing_character (cast `/Game/BIOPUNK/Core/BP_TestingCharacter` OtherActor))
  (`Interactable.BP_Interact` _asbp_testing_character))

(event `self.BP_Interact`
  (params (Interactor :type "Actor Object Reference"))
  ;[0 0 0] Cura subito al momento, non la mettiamo nell'inventario
  (bind _asbp_testing_character (cast `/Game/BIOPUNK/Core/BP_TestingCharacter` Interactor))
  (bind _bp_healthcomponent (`/Game/BIOPUNK/Core/BP_TestingCharacter.BP_HealthComponent` _asbp_testing_character))
  (`HealthComponent.SetHealth` _bp_healthcomponent (+ (`HealthComponent.GetHealth` _bp_healthcomponent) (`self.HealAmount`)))
  ;[0 0 0] RESPAWN CURA
  (`self.SetActive` false)
  (`KismetSystemLibrary.Delay` (`self.RespawnTime`))
  (`self.SetActive` true))

(fn `SetActive`
  (params (Active :type Boolean))
  (`self.SetActorHiddenInGame` (not Active))
  (`self.SetActorEnableCollision` (`local.Active`))
  (`self.SetActorTickEnabled` (`local.Active`)))

(fn `UserConstructionScript`)