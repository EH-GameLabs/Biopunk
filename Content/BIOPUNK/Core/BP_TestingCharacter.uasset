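; Testing player character for BIOPUNK melee combat, with stamina-gated sprint, combo attacks and dash, plus an ability montage, target lock and pause.
; Frenzy bar phases set damage and unlock longer combos and the ability; hits and perfect dodges raise the bar, damage taken lowers it.
; Perfect dashes also refund stamina and bend global time dilation.
; Socket-to-socket box sweeps and a radial Explode damage BP_BiopunkDummy targets.
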(event `EnhancedInput|/Game/BIOPUNK/Input/InputAction/IA_Ability`
  (params (ActionValue :type Boolean) (ElapsedSeconds :type "Float (double-precision)") (TriggeredSeconds :type "Float (double-precision)") (InputAction :type "InputAction Object Reference" :default "/Game/BIOPUNK/Input/InputAction/IA_Ability.IA_Ability"))
  (bind _returnvalue (`self.GetController`))
  (:`Triggered`
    (if (`self.Has Ability`)
      (`SceneComponent.SetHiddenInGame` (`self.Weapon`) true false)
      (if (not (`Controller.IsMoveInputIgnored` _returnvalue))
        (`Controller.SetIgnoreMoveInput` _returnvalue true))
      (set `self.bIsDashing` true)
      (`|PlayMontage` (`self.Mesh`) (`self.AbilityMontage`)
        (:`OnCompleted`
          (`Controller.SetIgnoreMoveInput` (`self.GetController`) false)
          (`SceneComponent.SetHiddenInGame` (`self.Weapon`) false false)
          (set `self.bIsDashing` false))))))

(event `EnhancedInput|/Game/BIOPUNK/Input/InputAction/IA_ActivateLastFrenzyPhase`
  (params (ActionValue :type Boolean) (ElapsedSeconds :type "Float (double-precision)") (TriggeredSeconds :type "Float (double-precision)") (InputAction :type "InputAction Object Reference" :default "/Game/BIOPUNK/Input/InputAction/IA_ActivateLastFrenzyPhase.IA_ActivateLastFrenzyPhase"))
  (:`Triggered`
    (`FrenzyComponent.ActivateLastPhase` (`self.Frenzy`))))

(event `StartRegen`
  (`KismetSystemLibrary.K2_ClearAndInvalidateTimerHandle` (`self.RegenTimerHandle`))
  (`KismetSystemLibrary.RetriggerableDelay` 2.0)
  (bind _returnvalue (`KismetSystemLibrary.K2_SetTimerDelegate` (delegate `RegenStamina`) 0.0001 true true))
  (set `self.RegenTimerHandle` _returnvalue))

(event `EnhancedInput|/Game/BIOPUNK/Input/InputAction/IA_Run`
  (params (ActionValue :type Boolean) (ElapsedSeconds :type "Float (double-precision)") (TriggeredSeconds :type "Float (double-precision)") (InputAction :type "InputAction Object Reference" :default "/Game/BIOPUNK/Input/InputAction/IA_Run.IA_Run"))
  (bind _charactermovement (`self.CharacterMovement`))
  (:`Triggered`
    (if (and (!= (`CharacterMovementComponent.GetLastUpdateVelocity` _charactermovement) (0.0 0.0 0.0)) (`NavMovementComponent.IsMovingOnGround` _charactermovement))
      (`self.UseStamina` (* 2.5 (`GameplayStatics.GetWorldDeltaSeconds`)))))
  (:`Started`
    (set `CharacterMovementComponent.MaxWalkSpeed` (`self.RunningSpeed`) (`self.CharacterMovement`)))
  (:`Completed`
    (set `CharacterMovementComponent.MaxWalkSpeed` (`self.WalkingSpeed`) (`self.CharacterMovement`))))

(event `RegenStamina`
  (if (>= (`self.CurrentStamina`) (`self.MaxStamina`))
    (`KismetSystemLibrary.K2_ClearAndInvalidateTimerHandle` (`self.RegenTimerHandle`))
    (else
      (set `self.CurrentStamina` (`KismetMathLibrary.FMin` (+ (`self.CurrentStamina`) (* (`GameplayStatics.GetWorldDeltaSeconds`) 10.0)) (`self.MaxStamina`))))))

(event `EnhancedInput|/Game/Input/Actions/IA_Jump`
  (params (ActionValue :type Boolean) (ElapsedSeconds :type "Float (double-precision)") (TriggeredSeconds :type "Float (double-precision)") (InputAction :type "InputAction Object Reference" :default "/Game/Input/Actions/IA_Jump.IA_Jump"))
  (:`Triggered`
    (if (not (`AnimInstance.IsAnyMontagePlaying` (`SkeletalMeshComponent.GetAnimInstance` (`self.Mesh`))))
      (`self.Jump`))))

(event `EnhancedInput|/Game/BIOPUNK/Input/InputAction/IA_TargetLock`
  (params (ActionValue :type Boolean) (ElapsedSeconds :type "Float (double-precision)") (TriggeredSeconds :type "Float (double-precision)") (InputAction :type "InputAction Object Reference" :default "/Game/BIOPUNK/Input/InputAction/IA_TargetLock.IA_TargetLock"))
  (:`Triggered`
    (`KismetSystemLibrary.PrintString` "Trying to lock")
    (`self.ToggleTargetLock`)))

(event `EnhancedInput|/Game/Variant_Combat/Input/Actions/IA_ComboAttack`
  (params (ActionValue :type Boolean) (ElapsedSeconds :type "Float (double-precision)") (TriggeredSeconds :type "Float (double-precision)") (InputAction :type "InputAction Object Reference" :default "/Game/Variant_Combat/Input/Actions/IA_ComboAttack.IA_ComboAttack"))
  (bind _returnvalue (`self.GetController`))
  (:`Started`
    (if (and (`NavMovementComponent.IsMovingOnGround` (`self.CharacterMovement`)) (`self.CanAttack`))
      (bind _outcome (`self.UseStamina` 5.0))
      (if _outcome
        (if (not (`Controller.IsMoveInputIgnored` _returnvalue))
          (`Controller.SetIgnoreMoveInput` _returnvalue true))
        (set `self.bIsDashing` true)
        (set `self.CanAttack` false)
        (`|PlayMontage` (`self.Mesh`) (`|GetArrayItem` (`self.AnimationsList`) (`self.ComboCounter`))
          (:`then`
            (if (`self.HasCombo`)
              (bind _result (`/Engine/EditorBlueprintResources/StandardMacros.IncrementInt` (`self.ComboCounter`))
                (:`  `
                  (set `self.ComboCounter` (mod _result (`KismetArrayLibrary.Array_Length` (`self.AnimationsList`))))))
              (else
                (bind _result_2 (`/Engine/EditorBlueprintResources/StandardMacros.IncrementInt` (`self.ComboCounter`))
                  (:`  `
                    (set `self.ComboCounter` (mod _result_2 2)))))))
          (:`OnCompleted`
            (set `self.CanAttack` true)
            (set `self.ComboCounter` 0)
            (`Controller.SetIgnoreMoveInput` (`self.GetController`) false)))))))

(event `PerfectDash`
  (bind _frenzy (`self.Frenzy`))
  (`self.GainStamina` (`self.DashCost`))
  (`FrenzyComponent.IncreaseBar` _frenzy (`FrenzyComponent.IncreaseBarOnPerfectDodge` _frenzy))
  ;[0 0 0] Durata uguale al tempo di dash
  (`TimelineComponent.SetPlayRate` (`self.Timeline DASH`) (/ (`TimelineComponent.GetTimelineLength` (`self.Timeline DASH`)) (`self.DashTime`)))
  ;[0 0 0] Cambiamento di GlobalTimeDilation
  (bind (_direction _newtrack_0) (`Timeline|Timeline DASH` :!via `PlayFromStart`)
    (:`Update`
      (`GameplayStatics.SetGlobalTimeDilation` _newtrack_0))
    (:`Finished`
      (`GameplayStatics.SetGlobalTimeDilation` 1.0))))

(event `self.ReceiveBeginPlay`
  (add `FrenzyComponent.OnBarChangedDelegate` (`self.Frenzy`) (delegate `TEST`))
  (set `self.BarDamage` (`.DamageMultiplier` (break `BarData` (`|GetArrayItem` (`FrenzyComponent.BarStats` (`self.Frenzy`)) (stale `TEST` index)))))
  (set `CharacterMovementComponent.MaxWalkSpeed` (`self.WalkingSpeed`) (`self.CharacterMovement`))
  (set `self.CurrentStamina` (`self.MaxStamina`)))

(event `TEST`
  (params (index :type Integer))
  (bind ((`DamageMultiplier` _damagemultiplier) (`HasCombo` _hascombo) (`HasAbility` _hasability)) (break `BarData` (`|GetArrayItem` (`FrenzyComponent.BarStats` (`self.Frenzy`)) index)))
  (if (!= index 2)
    (set `self.HasCombo` _hascombo :!label _label)
    (set `self.BarDamage` _damagemultiplier)
    (set `self.Has Ability` _hasability)
    (`KismetSystemLibrary.PrintString` "Hello")
    (elif (`FrenzyComponent.IsLastPhaseActive` (`self.Frenzy`))
      (goto _label))))

(event `self.Health.OnTakeDamage`
  (params (Damage :type Integer))
  ;[0 0 0] OnTakeDamage Delegate
  (`self.RemoveFrenzy`))

(event `self.Health.OnHealthChange`
  (params (NewHealth :type Integer))
  ;[0 0 0] OnHealthChange Delegate
)

(event `self.Health.OnDie`
  ;[0 0 0] OnDie Delegate
  (`KismetSystemLibrary.PrintString` "On DIE"))

(event `self.ReceiveTick`
  (params (DeltaSeconds :type "Float (single-precision)")))

(event `self.DoDash`
  ;[0 0 0] Dash Section
  (`parent.DoDash`)
  (`self.Dash`))

(event `Key|Escape`
  (params (Key :type "Key Structure"))
  (:`Pressed`
    (`self.Pause` :!label _label_2)))

(event `self.Frenzy.OnDamageMultiplierChanged`
  (params (NewMult :type "Float (single-precision)"))
  (set `HealthComponent.DamageMultiplier` NewMult (`self.Health`))
  (`KismetSystemLibrary.PrintString` (`KismetStringLibrary.Concat_StrStr` "New Damage Mult: " (`KismetStringLibrary.Conv_DoubleToString` NewMult)))
  (`FrenzyComponent.TriggerBarChange` (`self.Frenzy`) 2))

(event `Key|P`
  (params (Key :type "Key Structure"))
  (:`Pressed`
    (goto _label_2)))

(fn `CheckDashDir`
  (bind (_velocity_x _velocity_y) (`KismetMathLibrary.BreakVector` (`MovementComponent.Velocity` (`self.CharacterMovement`))))
  (bind (_velocity_x_2 _velocity_y_2) (`KismetMathLibrary.BreakVector` (`MovementComponent.Velocity` (`self.CharacterMovement`))))
  (bind _velocity_x_3 (`KismetMathLibrary.BreakVector` (`MovementComponent.Velocity` (`self.CharacterMovement`))))
  (if (> (`KismetMathLibrary.Abs` _velocity_x_2) (`KismetMathLibrary.Abs` _velocity_y_2))
    (if (> _velocity_x_3 0.0)
      (set `self.DashDir` "NewEnumerator0")
      (else
        (set `self.DashDir` "NewEnumerator1")))
    (elif (> _velocity_y 0.0)
      (set `self.DashDir` "NewEnumerator3")
      (else
        (set `self.DashDir` "NewEnumerator2")))))

(fn `Explode`
  (locals (HasHit :type Boolean) (Impulse :type "Float (double-precision)" :default 1000.0))
  (bind _explosionsize (`self.ExplosionSize`))
  (bind _returnvalue (`PrimitiveComponent.GetCenterOfMass` (`self.Mesh`) "None"))
  (bind _outhits (`KismetSystemLibrary.SphereTraceMulti` :`Start` _returnvalue :`End` _returnvalue :`Radius` _explosionsize :`TraceChannel` "TraceTypeQuery1" :`DrawTime` 0.5))
  (for _array_element _outhits
    (bind (_bblockinghit _binitialoverlap _time _distance _location _impactpoint _normal _impactnormal _physmat _hitactor) (`GameplayStatics.BreakHitResult` _array_element))
    (if (`KismetSystemLibrary.DoesImplementInterface` _hitactor "/Script/BioPunk.CombatDamageable")
      (bind _asbp_biopunk_dummy (cast `/Game/BIOPUNK/AI/BP_BiopunkDummy` _hitactor))
      (`CombatDamageable.ApplyDamage` _asbp_biopunk_dummy (* (`self.BarDamage`) (`self.AbilityDamage`)) null _impactpoint (* (`KismetMathLibrary.Normal` (- _impactpoint (`self.K2_GetActorLocation`))) (`local.Impulse`)))
      (set `local.HasHit` true)))
  (`KismetSystemLibrary.DrawDebugSphere` _returnvalue _explosionsize 12 (`KismetMathLibrary.SelectColor` (struct :`G` 1.0 :`A` 1.0) (struct :`R` 1.0 :`A` 1.0) (`local.HasHit`)) 0.5))

(fn `GainStamina`
  (params (Amount :type "Float (double-precision)"))
  (set `self.CurrentStamina` (`KismetMathLibrary.FMin` (+ Amount (`self.CurrentStamina`)) (`self.MaxStamina`))))

(fn `Pause`
  (bind _returnvalue (`GameplayStatics.GetPlayerController` 0))
  (bind _hud_canva (`/Game/BIOPUNK/UI/HUD_BioPunk.HUD_Canva` (`/Game/BIOPUNK/BFL_BioPunk.GetHUD`)))
  (cast `/Game/BIOPUNK/UI/WBP_HUD` (`/Game/BIOPUNK/UI/WBP_Canva.CurrentActiveWidget` _hud_canva))
  (`/Game/BIOPUNK/UI/WBP_Canva.PushWidgetOnCanva` _hud_canva "/Game/BIOPUNK/UI/WBP_Pause.WBP_Pause_C" true)
  (`GameplayStatics.SetGamePaused` true)
  (`WidgetBlueprintLibrary.SetInputMode_UIOnlyEx` _returnvalue null)
  (set `PlayerController.bShowMouseCursor` true _returnvalue))

(fn `RemoveFrenzy`
  (bind _frenzy (`self.Frenzy`))
  (`FrenzyComponent.DecreaseBar` _frenzy (`FrenzyComponent.DecreaseBarOnTakeDamage` _frenzy)))

(fn `SetPerfectDash`
  (params (Active :type Boolean))
  (set `self.IsPerfectDash` Active))

(fn `TraceStart`
  (set `self.TopSocketPos` (`SceneComponent.GetSocketLocation` (`self.Weapon`) (`self.TopSocket Name`)))
  (set `self.BottomSocketPos` (`SceneComponent.GetSocketLocation` (`self.Weapon`) (`self.BottomSocket Name`)))
  (`KismetArrayLibrary.Array_Clear` (`self.HitActors`)))

(fn `TraceTick`
  (locals (CurrentTop :type "Vector Structure" :default (0.0 0.0 0.0)) (CurrentBottom :type "Vector Structure" :default (0.0 0.0 0.0)))
  (bind _tracesize (`self.TraceSize`))
  (bind _frenzy (`self.Frenzy`))
  (bind _currenttop (`local.CurrentTop`))
  (bind _currentbottom (`local.CurrentBottom`))
  (bind _hitactors (`self.HitActors`))
  (set `local.CurrentTop` (`SceneComponent.GetSocketLocation` (`self.Weapon`) (`self.TopSocket Name`)))
  (set `local.CurrentBottom` (`SceneComponent.GetSocketLocation` (`self.Weapon`) (`self.BottomSocket Name`)))
  (bind _outhits (`KismetSystemLibrary.BoxTraceMulti` :`Start` (/ (+ (`self.BottomSocketPos`) (`self.TopSocketPos`)) 2.0) :`End` (/ (+ (`local.CurrentBottom`) (`local.CurrentTop`)) 2.0) :`HalfSize` (`KismetMathLibrary.MakeVector` (/ (`KismetMathLibrary.Vector_Distance` _currentbottom _currenttop) 2.0) _tracesize _tracesize) :`Orientation` (`KismetMathLibrary.FindLookAtRotation` _currenttop _currentbottom) :`TraceChannel` "TraceTypeQuery1" :`DrawDebugType` "ForDuration" :`DrawTime` 0.5))
  (for _array_element _outhits
    (bind (_bblockinghit _binitialoverlap _time _distance _location _impactpoint _normal _impactnormal _physmat _hitactor) (`GameplayStatics.BreakHitResult` _array_element))
    (if (not (`KismetArrayLibrary.Array_Contains` _hitactors _hitactor))
      (`KismetSystemLibrary.PrintString` (`KismetSystemLibrary.GetDisplayName` _hitactor))
      (`KismetArrayLibrary.Array_AddUnique` _hitactors _hitactor)
      (if (`KismetSystemLibrary.DoesImplementInterface` _hitactor "/Script/BioPunk.CombatDamageable")
        (bind _asbp_biopunk_dummy (cast `/Game/BIOPUNK/AI/BP_BiopunkDummy` _hitactor))
        (`CombatDamageable.ApplyDamage` _asbp_biopunk_dummy (`self.BarDamage`) null _impactpoint (`KismetMathLibrary.Vector_Zero`))
        (`FrenzyComponent.IncreaseBar` _frenzy (`FrenzyComponent.IncreaseBarOnHit` _frenzy)))))
  (set `self.TopSocketPos` (`local.CurrentTop`))
  (set `self.BottomSocketPos` (`local.CurrentBottom`)))

(fn `UserConstructionScript`)

(fn `UseStamina`
  (params (StaminaInput :type "Float (double-precision)"))
  (returns (Outcome :type Boolean))
  (if (<= StaminaInput (`self.CurrentStamina`))
    (`self.StartRegen`)
    (set `self.CurrentStamina` (- (`self.CurrentStamina`) (`local.StaminaInput`)))
    (return true)
    (else
      (`KismetSystemLibrary.PrintString` "Not enough stamina")
      (return false))))