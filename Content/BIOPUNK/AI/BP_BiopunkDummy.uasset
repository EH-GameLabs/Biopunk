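; BP_BiopunkDummy is a targetable AI dummy with a patrol flag that spawns a directional Niagara effect when damaged.
; A sphere overlap writes the player and their last position to the Blackboard.
; A toggleable perfect-dodge collider sets the player's perfect-dash state while overlapped.
; Helpers tint the mesh material and apply per-actor hit stop by zeroing CustomTimeDilation until a timer calls the restore.
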(event `self.ReceivedDamage`
  (params (Damage :type "Float (single-precision)") (ImpactPoint :type "Vector Structure (by ref)") (DamageDirection :type "Vector Structure (by ref)"))
  (`NiagaraFunctionLibrary.SpawnSystemAtLocation` "/Game/Variant_Combat/VFX/NS_Damage.NS_Damage" ImpactPoint (`KismetMathLibrary.Conv_VectorToRotator` DamageDirection)))

(event `self.Sphere Collision.OnComponentBeginOverlap`
  (params (OverlappedComponent :type "PrimitiveComponent Object Reference") (OtherActor :type "Actor Object Reference") (OtherComp :type "PrimitiveComponent Object Reference") (OtherBodyIndex :type Integer) (bFromSweep :type Boolean) (SweepResult :type "HitResult Structure (by ref)"))
  (bind _asbp_testing_character (cast `/Game/BIOPUNK/Core/BP_TestingCharacter` OtherActor))
  (`BlackboardComponent.SetValueAsObject` (`AIBlueprintHelperLibrary.GetBlackboard` null) "Player" _asbp_testing_character)
  (`BlackboardComponent.SetValueAsVector` (`AIBlueprintHelperLibrary.GetBlackboard` null) "LastPlayerPos" (`self.K2_GetActorLocation` _asbp_testing_character)))

(event `self.Perfect Dodge Collision.OnComponentBeginOverlap`
  (params (OverlappedComponent :type "PrimitiveComponent Object Reference") (OtherActor :type "Actor Object Reference") (OtherComp :type "PrimitiveComponent Object Reference") (OtherBodyIndex :type Integer) (bFromSweep :type Boolean) (SweepResult :type "HitResult Structure (by ref)"))
  (bind _asbp_testing_character (cast `/Game/BIOPUNK/Core/BP_TestingCharacter` OtherActor))
  (`/Game/BIOPUNK/Core/BP_TestingCharacter.SetPerfectDash` _asbp_testing_character true))

(event `self.Perfect Dodge Collision.OnComponentEndOverlap`
  (params (OverlappedComponent :type "PrimitiveComponent Object Reference") (OtherActor :type "Actor Object Reference") (OtherComp :type "PrimitiveComponent Object Reference") (OtherBodyIndex :type Integer))
  (bind _asbp_testing_character (cast `/Game/BIOPUNK/Core/BP_TestingCharacter` OtherActor))
  (`/Game/BIOPUNK/Core/BP_TestingCharacter.SetPerfectDash` _asbp_testing_character false))

(fn `ChangeColor`
  (params (ParameterValue :type "LinearColor Structure"))
  (`MeshComponent.SetColorParameterValueOnMaterials` (`self.Mesh`) "Color" ParameterValue))

(fn `EndHitStop`
  (set `self.CustomTimeDilation` 1.0))

(fn `GetPatrolStatus`
  (returns (ReturnValue :type Boolean))
  (return (`self.HasToPatrol`)))

(fn `GetTargetLocation`
  (returns (ReturnValue :type "Vector Structure"))
  (return (`SceneComponent.K2_GetComponentLocation` (`self.Scene`))))

(fn `IsTargetable`
  (returns (ReturnValue :type Boolean))
  (return true))

(fn `SetPerfectDodgeCollision`
  (params (Active :type Boolean))
  (if Active
    (`PrimitiveComponent.SetCollisionEnabled` (`self.Perfect Dodge Collision`) "QueryAndPhysics")
    (else
      (`PrimitiveComponent.SetCollisionEnabled` (`self.Perfect Dodge Collision`) "NoCollision"))))

(fn `StartHitStop`
  (params (Duration :type "Float (double-precision)"))
  (set `self.CustomTimeDilation` 0.0)
  (`KismetSystemLibrary.K2_SetTimer` null "EndHitStop" Duration))

(fn `UserConstructionScript`)