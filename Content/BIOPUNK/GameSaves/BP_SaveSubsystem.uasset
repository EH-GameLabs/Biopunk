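; BP_SaveSubsystem is a save subsystem that stores and restores the player's transform.
; It calls LoadGame on initialization, and both save and load run their parent implementations and print a debug message.
; SaveGame captures the GameManager player's transform into PlayerPos after the parent save call.
; HandleLoadGame teleports the player to PlayerPos, but nothing in this file calls it.
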(event `self.ReceiveInitialize`
  (`self.LoadGame`))

(event `self.SaveGame`
  (`parent.SaveGame`)
  (`self.HandleSaveGame`)
  (`KismetSystemLibrary.PrintString` "GameSaved"))

(event `self.LoadGame`
  (`parent.LoadGame`)
  (`KismetSystemLibrary.PrintString` "LoadGame"))

(fn `HandleLoadGame`
  (locals (LocalPlayer :type "/Game/BIOPUNK/Core/BP_TestingCharacter Object Reference"))
  (set `local.LocalPlayer` (`/Game/BIOPUNK/Core/BP_GameManager.GetPlayer` (`/Game/BIOPUNK/BFL_BioPunk.GetGameManager`)))
  (`Actor.K2_SetActorTransform` (`local.LocalPlayer`) (`self.PlayerPos`) false true))

(fn `HandleSaveGame`
  (locals (LocalPlayer :type "/Game/BIOPUNK/Core/BP_TestingCharacter Object Reference"))
  (set `local.LocalPlayer` (`/Game/BIOPUNK/Core/BP_GameManager.GetPlayer` (`/Game/BIOPUNK/BFL_BioPunk.GetGameManager`)))
  (set `self.PlayerPos` (`Actor.GetTransform` (`local.LocalPlayer`))))